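; BatBP is a bat power that knocks another player character away on right mouse press.
; A DoOnce and a Couldown flag gate a short debug-drawn sphere trace for pawns, forward from component R.
; A hit Principal_Perso is launched along HitBat's forward vector with added lift, then R is destroyed.
; It sets a timer for "Spam", but that function, any DoOnce reset and any Couldown reset are absent here.
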(event Input|MouseEvents|RightMouseButton
  (params (Key :type Key%20Structure :default "None"))
  (bind _hit_bat (Variables|Default|Gethit%20bat))
  (bind _r (Variables|Default|Getr))
  (bind _returnvalue (Transformation|GetWorldLocation _r))
  (bind _returnvalue_2 (Transformation|GetWorldRotation _hit_bat))
  (bind _returnvalue_3 (Math|Vector|GetForwardVector _returnvalue_2))
  (bind _returnvalue_4 (* _returnvalue_3 2e+03))
  (:Pressed
    (Utilities|FlowControl|DoOnce false
      (:Completed
        (if (Variables|Default|Getcouldown)
          (Utilities|Time|SetTimerbyFunctionName 0 "Spam" 1.0)
          (Variables|Default|Setcouldown false)
          (bind (_outhit _returnvalue_5) (Collision|SphereTraceForObjects _returnvalue (+ _returnvalue (* (Math|Vector|GetForwardVector (Transformation|GetWorldRotation _r)) 1.5e+02)) 5e+01 (Utilities|Array|MakeArray "ObjectTypeQuery3") false 0 "ForDuration"))
          (if _returnvalue_5
            (bind _asprincipal_perso (Utilities|Casting|CastToPrincipal_Perso (.HitActor (Collision|BreakHitResult _outhit))))
            (Character|LaunchCharacter _asprincipal_perso (Math|Vector|MakeVector (.x _returnvalue_4) (.y _returnvalue_4) (+ (.z _returnvalue_4) 1e+03)) false false)
            (Components|DestroyComponent (Variables|Default|Getr))))))))

(fn ConstructionScript)