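; Rocket power-up actor that switches player control to a rocket pawn when BP_Player1 overlaps its box.
; It spawns BP_Pawn_Rocket at the player's location and has player controller 0 possess it.
; After a very short delay, it sets the view target to a CameraActor found in the level.
; That camera step runs on any overlap, even when the player cast fails.
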(event OnComponentBeginOverlap(Box)
  (params (OverlappedComponent :type Primitive%20Component%20Object%20Reference) (OtherActor :type Actor%20Object%20Reference) (OtherComp :type Primitive%20Component%20Object%20Reference) (OtherBodyIndex :type Integer) (bFromSweep :type Boolean) (SweepResult :type Hit%20Result%20Structure%20%28by%20ref%29))
  (Utilities|FlowControl|Sequence
    (:then_0
      (bind _asbp_player_1 (Utilities|Casting|CastToBP_Player1 OtherActor))
      (bind _returnvalue (Game|SpawnActorfromClass "/Game/Manu/BP_Pawn_Rocket.BP_Pawn_Rocket_C" (Math|Transform|MakeTransform (Transformation|GetActorLocation _asbp_player_1) "0, 0, 0" "1.000000,1.000000,1.000000") "Undefined" "MultiplyWithRoot" 0 0))
      (Pawn|Possess (Game|GetPlayerController 0) _returnvalue))
    (:then_1
      (Utilities|FlowControl|Delay 0.01)
      (bind _returnvalue_2 (Actor|GetActorOfClass "/Script/Engine.CameraActor"))
      (Variables|Default|SetNew%20View%20Target _returnvalue_2)
      (Game|Player|SetViewTargetwithBlend (Game|GetPlayerController 0) (Variables|Default|GetNew%20View%20Target) 0.0 "VTBlend_Linear" 0.0 false))))

(fn ConstructionScript)