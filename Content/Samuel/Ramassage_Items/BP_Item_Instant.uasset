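; BP_Item_Instant is a pickup item that applies its effect to the player as soon as it is interacted with.
; The construction script sets the item's mesh from the ItemModelToPlace variable.
; On InteractionFunction, it identifies the item by its mesh, setting the ChampignonActiver (mushroom) flag on BP_ThirdPersonCharacter for SM_ChamferCube.
; It prints a pickup message and, if the character cast succeeds, destroys itself a tick later.
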(event EventBeginPlay)

(event Collision|EventActorBeginOverlap
  (params (OtherActor :type Actor%20Object%20Reference)))

(event EventTick
  (params (DeltaSeconds :type Float%20%28single-precision%29)))

(event EventInteractionFunction
  (Development|PrintString "item picked")
  (bind _asbp_third_person_character (Utilities|Casting|CastToBP_ThirdPersonCharacter (Game|GetPlayerCharacter 0)))
  (if (== (Variables|/Script/Engine.StaticMeshComponent|GetStaticMesh (Variables|Default|GetItemModel)) "/Game/Base_Asset/LevelPrototyping/Meshes/SM_ChamferCube.SM_ChamferCube")
    (Variables|/Game/Base_Asset/ThirdPerson/Blueprints/BP_ThirdPersonCharacter.BP_ThirdPersonCharacter_C|SetChampignonActiver _asbp_third_person_character true))
  (Utilities|FlowControl|DelayUntilNextTick)
  (Actor|DestroyActor))

(fn ConstructionScript
  (Components|StaticMesh|SetStaticMesh (Variables|Default|GetItemModel) (Variables|Default|GetItemModelToPlace)))